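; BP_Boat is a boat driven by Forward and Right input events through physics on its Board component.
; Forward adds an acceleration-mode force along the actor's forward vector, flattened to horizontal and scaled by ForwardSpeed.
; Right adds torque around the control rotation's up vector, scaled by RataSpeed.
; Both events print their direction vectors for debugging, and a camera-to-Sphere position snap is left disconnected.
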(event Custom|Forward
  (params (forwardValue :type Float%20%28single-precision%29))
  (bind _returnvalue (Transformation|GetActorRotation))
  (bind _returnvalue_2 (Math|Vector|GetForwardVector _returnvalue))
  (bind (_x _y) (Math|Vector|BreakVector _returnvalue_2))
  (bind _returnvalue_3 (Math|Vector|MakeVector _x _y 0.0))
  ;[1 1 1] 前进
  (Development|PrintString (Utilities|String|Append "ForwardVec：" (Utilities|String|ToString(Vector) _returnvalue_3)) true true "(R=1.000000,G=0.102242,B=0.000000,A=1.000000)")
  (Physics|AddForce (Variables|Default|GetBoard) (* (* _returnvalue_3 (Variables|Default|GetForwardSpeed)) forwardValue) "None" true))

(event Custom|Right
  (params (rightValue :type Float%20%28single-precision%29))
  (bind _returnvalue (Pawn|GetControlRotation :!class /Script/Engine.Pawn))
  (bind _returnvalue_2 (Math|Vector|GetUpVector _returnvalue))
  ;[1 1 1] 转向
  (Development|PrintString (Utilities|String|Append "UpVec：" (Utilities|String|ToString(Vector) _returnvalue_2)) true true "(R=1.000000,G=0.102242,B=0.000000,A=1.000000)")
  (Class|PrimitiveComponent|AddTorqueinRadians (Variables|Default|GetBoard) (* (* _returnvalue_2 (Variables|Default|GetRataSpeed)) rightValue) "None" true))

(fn ConstructionScript)