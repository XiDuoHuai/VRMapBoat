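; BP_BoatHide is a companion actor that shadows the boat, showing a Cube component that moves and turns with it.
; On BeginPlay it caches the first BP_Boat found in the level and makes the Cube visible.
; Every Tick it copies the boat's location and rotation onto itself without sweeping, following by transform copy rather than attachment.
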(event EventBeginPlay
  (bind _outactors (Actor|GetAllActorsOfClass "/Game/VRContent/BluePrint/Boat/BP_Boat.BP_Boat_C"))
  (Variables|Default|SetBP_Boat (Utilities|Array|Get(acopy) _outactors))
  (Rendering|SetVisibility (Variables|Default|GetCube) true false))

(event Collision|EventActorBeginOverlap
  (params (OtherActor :type Actor%20Object%20Reference)))

(event EventTick
  (params (DeltaSeconds :type Float%20%28single-precision%29))
  (Transformation|SetActorLocation (Transformation|GetActorLocation (Variables|Default|GetBP_Boat)) false false)
  (Transformation|SetActorRotation (Transformation|GetActorRotation (Variables|Default|GetBP_Boat))))

(fn ConstructionScript)