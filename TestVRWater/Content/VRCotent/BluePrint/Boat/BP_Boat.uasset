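; BP_Boat is a physics-driven boat with forward/reverse and turning control.
; Forward pushes the Board component along the control rotation's forward vector, scaled by ForwardSpeed and input, and prints that vector for debugging.
; Right applies torque around the control rotation's up vector, scaled by RataSpeed and input.
; Both use acceleration change to ignore mass; logic pinning Camera to Sphere is disconnected.
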(event Custom|Forward
  (params (forwardValue :type Float%20%28single-precision%29))
  (bind _returnvalue (Pawn|GetControlRotation :!class /Script/Engine.Pawn))
  (bind _returnvalue_2 (Math|Vector|GetForwardVector _returnvalue))
  ;[1 1 1] 前进
  (Development|PrintString (Utilities|String|ToString(Vector) _returnvalue_2))
  (Physics|AddForce (Variables|Default|GetBoard) (* (* _returnvalue_2 (Variables|Default|GetForwardSpeed)) forwardValue) "None" true))

(event Custom|Right
  (params (rightValue :type Float%20%28single-precision%29))
  ;[1 1 1] 转向
  (Class|PrimitiveComponent|AddTorqueinRadians (Variables|Default|GetBoard) (* (* (Math|Vector|GetUpVector (Pawn|GetControlRotation :!class /Script/Engine.Pawn)) (Variables|Default|GetRataSpeed)) rightValue) "None" true))

(fn ConstructionScript)