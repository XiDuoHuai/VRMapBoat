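; VR boat paddle that drives a referenced BPBoat while either blade box overlaps a WaterBody.
; Overlaps open per-side Tick gates that pass each blade's horizontal per-frame movement to Forward and cylinder pitch to Right, turning opposite the stroking side.
; Z=1 in the previous position marks a stroke start, but right-side exit resets the left value.
; CalDirection sits only in unexecuted nodes, so thrust ignores stroke direction.
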(event OnComponentBeginOverlap(Capsule)
  (params (OverlappedComponent :type Primitive%20Component%20Object%20Reference) (OtherActor :type Actor%20Object%20Reference) (OtherComp :type Primitive%20Component%20Object%20Reference) (OtherBodyIndex :type Integer) (bFromSweep :type Boolean) (SweepResult :type Hit%20Result%20Structure%20%28by%20ref%29)))

(event OnComponentEndOverlap(LeftBox)
  (params (OverlappedComponent :type Primitive%20Component%20Object%20Reference) (OtherActor :type Actor%20Object%20Reference) (OtherComp :type Primitive%20Component%20Object%20Reference) (OtherBodyIndex :type Integer))
  (bind _leftbox (Variables|Default|GetLeftBox))
  (bind _bp_boat (Variables|Default|GetBP_Boat))
  (bind _leftbox_2 (Variables|Default|GetLeftBox))
  (bind _returnvalue (Transformation|GetWorldLocation _leftbox))
  (bind _returnvalue_2 (Transformation|GetWorldLocation _leftbox_2))
  (bind (_x _y) (Math|Vector|BreakVector _returnvalue))
  (bind (_x_2 _y_2) (Math|Vector|BreakVector _returnvalue_2))
  ;[1 1 1] 左桨触水移动
  (Utilities|Casting|CastToWaterBody OtherActor)
  (Variables|Default|SetLeft_PreLocation "0, 0,1.000000")
  (Utilities|FlowControl|Gate true) ; enters at Close
)

(event OnComponentBeginOverlap(LeftBox)
  (params (OverlappedComponent :type Primitive%20Component%20Object%20Reference) (OtherActor :type Actor%20Object%20Reference) (OtherComp :type Primitive%20Component%20Object%20Reference) (OtherBodyIndex :type Integer) (bFromSweep :type Boolean) (SweepResult :type Hit%20Result%20Structure%20%28by%20ref%29))
  (bind _leftbox (Variables|Default|GetLeftBox))
  (bind _bp_boat (Variables|Default|GetBP_Boat))
  (bind _leftbox_2 (Variables|Default|GetLeftBox))
  (bind _returnvalue (Transformation|GetWorldLocation _leftbox))
  (bind _returnvalue_2 (Transformation|GetWorldLocation _leftbox_2))
  (bind (_x _y) (Math|Vector|BreakVector _returnvalue))
  (bind (_x_2 _y_2) (Math|Vector|BreakVector _returnvalue_2))
  ;[1 1 1] 左桨触水移动
  (Utilities|Casting|CastToWaterBody OtherActor)
  (Development|PrintString "l")
  (Utilities|FlowControl|Gate true) ; enters at Open
)

(event OnComponentBeginOverlap(RightBox)
  (params (OverlappedComponent :type Primitive%20Component%20Object%20Reference) (OtherActor :type Actor%20Object%20Reference) (OtherComp :type Primitive%20Component%20Object%20Reference) (OtherBodyIndex :type Integer) (bFromSweep :type Boolean) (SweepResult :type Hit%20Result%20Structure%20%28by%20ref%29))
  (bind _rightbox (Variables|Default|GetRightBox))
  (bind _rightbox_2 (Variables|Default|GetRightBox))
  (bind _bp_boat (Variables|Default|GetBP_Boat))
  (bind _returnvalue (Transformation|GetWorldLocation _rightbox))
  (bind _returnvalue_2 (Transformation|GetWorldLocation _rightbox_2))
  (bind (_x _y) (Math|Vector|BreakVector _returnvalue))
  (bind (_x_2 _y_2) (Math|Vector|BreakVector _returnvalue_2))
  ;[1 1 1] 右浆触水移动
  (Utilities|Casting|CastToWaterBody OtherActor)
  (Development|PrintString "r")
  (Utilities|FlowControl|Gate true) ; enters at Open
)

(event OnComponentEndOverlap(RightBox)
  (params (OverlappedComponent :type Primitive%20Component%20Object%20Reference) (OtherActor :type Actor%20Object%20Reference) (OtherComp :type Primitive%20Component%20Object%20Reference) (OtherBodyIndex :type Integer))
  (bind _rightbox (Variables|Default|GetRightBox))
  (bind _rightbox_2 (Variables|Default|GetRightBox))
  (bind _bp_boat (Variables|Default|GetBP_Boat))
  (bind _returnvalue (Transformation|GetWorldLocation _rightbox))
  (bind _returnvalue_2 (Transformation|GetWorldLocation _rightbox_2))
  (bind (_x _y) (Math|Vector|BreakVector _returnvalue))
  (bind (_x_2 _y_2) (Math|Vector|BreakVector _returnvalue_2))
  ;[1 1 1] 右浆触水移动
  (Utilities|Casting|CastToWaterBody OtherActor)
  (Variables|Default|SetLeft_PreLocation "0, 0,1.000000")
  (Utilities|FlowControl|Gate true) ; enters at Close
)

(event EventBeginPlay)

(event EventTick
  (params (DeltaSeconds :type Float%20%28single-precision%29))
  (bind _leftbox (Variables|Default|GetLeftBox))
  (bind _rightbox (Variables|Default|GetRightBox))
  (bind _rightbox_2 (Variables|Default|GetRightBox))
  (bind _bp_boat (Variables|Default|GetBP_Boat))
  (bind _bp_boat_2 (Variables|Default|GetBP_Boat))
  (bind _leftbox_2 (Variables|Default|GetLeftBox))
  (bind _returnvalue (Transformation|GetWorldLocation _rightbox))
  (bind _returnvalue_2 (Transformation|GetWorldLocation _leftbox))
  (bind _returnvalue_3 (Transformation|GetWorldLocation _leftbox_2))
  (bind _returnvalue_4 (Transformation|GetWorldLocation _rightbox_2))
  (bind (_x _y) (Math|Vector|BreakVector _returnvalue))
  (bind (_x_2 _y_2) (Math|Vector|BreakVector _returnvalue_2))
  (bind (_x_3 _y_3) (Math|Vector|BreakVector _returnvalue_3))
  (bind (_x_4 _y_4) (Math|Vector|BreakVector _returnvalue_4))
  (Utilities|FlowControl|Sequence
    (:then_0
      ;[1 1 1] 左桨触水移动
      (Utilities|FlowControl|Gate true
        (:Exit
          (if (== (.Z (Math|Vector|BreakVector (Variables|Default|GetLeft_PreLocation))) 1.0)
            (Variables|Default|SetLeft_PreLocation (Math|Vector|MakeVector _x_3 _y_3 0.0))
            (else
              (bind _output_get (Variables|Default|SetLeft_CurrLocation (Math|Vector|MakeVector _x_2 _y_2 0.0)))
              (if (not (== (Math|Vector|VectorLength (- (Variables|Default|GetLeft_PreLocation) _output_get)) 0.0))
                (Utilities|IsValid _bp_boat_2
                  (:Is%20Valid
                    (Default|Forward _bp_boat_2 (* 1.0 (Math|Vector|VectorLength (- (Variables|Default|GetLeft_PreLocation) _output_get))))
                    (Variables|Default|SetLeft_PreLocation (Variables|Default|GetLeft_CurrLocation))
                    ;[1 1 1] 左船桨控制船体右转
                    (Default|Right (Variables|Default|GetBP_Boat) (/ (- 9e+01 (.Pitch (Math|Rotator|BreakRotator (Transformation|GetWorldRotation (Variables|Default|GetCylinder))))) 9e+01))))))))))
    (:then_1
      ;[1 1 1] 右浆触水移动
      (Utilities|FlowControl|Gate true
        (:Exit
          (if (== (.Z (Math|Vector|BreakVector (Variables|Default|GetRight_PreLocation))) 1.0)
            (Variables|Default|SetRight_PreLocation (Math|Vector|MakeVector _x _y 0.0))
            (else
              (bind _output_get_2 (Variables|Default|SetRight_CurrLocation (Math|Vector|MakeVector _x_4 _y_4 0.0)))
              (if (not (== (Math|Vector|VectorLength (- _output_get_2 (Variables|Default|GetRight_PreLocation))) 0.0))
                (Utilities|IsValid _bp_boat
                  (:Is%20Valid
                    (Default|Forward _bp_boat (* 1.0 (Math|Vector|VectorLength (- _output_get_2 (Variables|Default|GetRight_PreLocation)))))
                    (Variables|Default|SetRight_PreLocation (Variables|Default|GetRight_CurrLocation))
                    ;[1 1 1] 右桨控制船体左转
                    (Default|Right (Variables|Default|GetBP_Boat) (* (/ (+ (.Pitch (Math|Rotator|BreakRotator (Transformation|GetWorldRotation (Variables|Default|GetCylinder)))) 9e+01) 9e+01) -1.0))))))))))))

(fn ConstructionScript)

(fn LeftHandleShake)

(fn RightHandleShake)

(fn CalDirection
  (params (Pre :type Vector) (Back :type Vector))
  (bind _returnvalue (Transformation|GetActorLocation))
  (bind _returnvalue_2 (- _returnvalue Back))
  (bind _returnvalue_3 (- _returnvalue Pre))
  (bind _returnvalue_4 (- _returnvalue_3 _returnvalue_2))
  (bind (_x _y) (Math|Vector|BreakVector _returnvalue_4))
  (bind _returnvalue_5 (Math|Vector|Normalize (Math|Vector|MakeVector _x _y 0.0)))
  (bind _x_2 (Math|Vector|BreakVector _returnvalue_5))
  (bind _returnvalue_6 (<= _x_2 0.0))
  (bind _returnvalue_7 (select _returnvalue_6 1 -1))
  ;[1 1 1] 前进返回-1 后退返回1
  (Development|PrintString (Utilities|String|ToString(Integer) _returnvalue_7))
  (return _returnvalue_7))